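; Actor component for puzzle-style static mesh objects that can have their position stored, be frozen in place, or be reset to the saved transform.
; Storing and freezing are mutually exclusive toggles that spend and refund limited Stores and Freezes on GameInst, showing a FadinTxt widget when blocked.
; BeginPlay derives the saved transform, optionally from a preset offset, and applies physics.
; SetColor colour-codes each state through the "Col" material parameter.
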(event EventBeginPlay
  (bind _returnvalue (Components|GetOwner))
  (bind _returnvalue_2 (Transformation|GetActorTransform _returnvalue))
  ;[1 1 1] Gets the Inital Position and colour codes the cubes
  (bind _output_get (Variables|Default|SetNothingSet (== (Variables|Default|GetInitalTransform) (Variables|Default|GetSavedTransform))))
  (if _output_get
    (Variables|Default|SetSavedTransform _returnvalue_2)
    (else
      (Variables|Default|SetSavedTransform (Math|Transform|ComposeTransforms _returnvalue_2 (Variables|Default|GetSavedTransform)))))
  (Variables|Default|SetInitalTransform _returnvalue_2)
  (bind _asstatic_mesh_actor (Utilities|Casting|CastToStaticMeshActor _returnvalue))
  (Physics|SetSimulatePhysics (Variables|/Script/Engine.StaticMeshActor|GetStaticMeshComponent _asstatic_mesh_actor) (Variables|Default|GetHasPhysics))
  (CallFunction|SetColor))

(event EventTick
  (params (DeltaSeconds :type Float%20%28single-precision%29)))

(fn SaveDeleteCurrentPos
  (bind _asgame_inst (Utilities|Casting|CastToGameInst (Game|GetGameInstance)))
  (if (Variables|Default|GetHasPhysics)
    (if (Variables|Default|GetNothingSet)
      (if (> (Variables|/Game/Blueprints/GameInst.GameInst_C|GetStores _asgame_inst) 0)
        (Math|Integer|DecrementInt (Variables|/Game/Blueprints/GameInst.GameInst_C|GetStores _asgame_inst)
          (:%20%20
            (Audio|PlaySound2D "/Game/Sounds/Audio/UnStore.UnStore" 1.0 1.0 0.0 0 0)
            (Variables|Default|SetSavedTransform (Transformation|GetActorTransform (Components|GetOwner)))
            (Variables|Default|SetNothingSet (not (Variables|Default|GetNothingSet)) :!label _label)
            (CallFunction|SetColor)))
        (else
          (bind _returnvalue (UserInterface|CreateWidget "/Game/UI/FadinTxt.FadinTxt_C"))
          (Default|GetContition _returnvalue false)
          (UserInterface|Viewport|AddtoViewport _returnvalue 0)))
      (else
        (Math|Integer|IncrementInt (Variables|/Game/Blueprints/GameInst.GameInst_C|GetStores _asgame_inst)
          (:%20%20
            (Audio|PlaySound2D "/Game/Sounds/Audio/StorePos.StorePos" 1.0 1.0 0.0 0 0)
            (Variables|Default|SetSavedTransform (Variables|Default|GetInitalTransform))
            (goto _label)))))
    (else
      (bind _returnvalue_2 (UserInterface|CreateWidget "/Game/UI/FadinTxt.FadinTxt_C"))
      (Default|GetContition _returnvalue_2 true)
      (UserInterface|Viewport|AddtoViewport _returnvalue_2 0))))

(fn FreezeUnfreeze
  (bind _asgame_inst (Utilities|Casting|CastToGameInst (Game|GetGameInstance)))
  (if (Variables|Default|GetNothingSet)
    (if (Variables|Default|GetHasPhysics)
      (if (> (Variables|/Game/Blueprints/GameInst.GameInst_C|GetFreezes _asgame_inst) 0)
        (Math|Integer|DecrementInt (Variables|/Game/Blueprints/GameInst.GameInst_C|GetFreezes _asgame_inst)
          (:%20%20
            (Audio|PlaySound2D "/Game/Sounds/Audio/SetFreeze.SetFreeze" 1.0 1.0 0.0 0 0)
            (bind _asstatic_mesh_actor (Utilities|Casting|CastToStaticMeshActor (Components|GetOwner) :!label _label))
            (bind _output_get (Variables|Default|SetHasPhysics (not (Variables|Default|GetHasPhysics))))
            (Physics|SetSimulatePhysics (Variables|/Script/Engine.StaticMeshActor|GetStaticMeshComponent _asstatic_mesh_actor) _output_get)
            (CallFunction|SetColor)))
        (else
          ;[1 1 1] Dispalyes why action cant be carried
          (bind _returnvalue (UserInterface|CreateWidget "/Game/UI/FadinTxt.FadinTxt_C"))
          (Default|GetContition _returnvalue false)
          (UserInterface|Viewport|AddtoViewport _returnvalue 0)))
      (else
        (Math|Integer|IncrementInt (Variables|/Game/Blueprints/GameInst.GameInst_C|GetFreezes _asgame_inst)
          (:%20%20
            (Audio|PlaySound2D "/Game/Sounds/Audio/UnFreeze.UnFreeze" 1.0 1.0 0.0 0 0)
            (goto _label)))))
    (else
      ;[1 1 1] displayes why action cant be carried
      (bind _returnvalue_2 (UserInterface|CreateWidget "/Game/UI/FadinTxt.FadinTxt_C"))
      (Default|GetContition _returnvalue_2 true)
      (UserInterface|Viewport|AddtoViewport _returnvalue_2 0))))

(fn ResetPos
  (Audio|PlaySound2D "/Game/Sounds/Audio/Reset.Reset" 0.2 0.5 0.0 0 0)
  (Transformation|SetActorTransform (Components|GetOwner) (Variables|Default|GetSavedTransform)))

(fn SetColor
  (bind _asstatic_mesh_actor (Utilities|Casting|CastToStaticMeshActor (Components|GetOwner)))
  (if (Variables|Default|GetHasPhysics)
    (if (Variables|Default|GetNothingSet)
      (Rendering|Material|SetVectorParameterValueonMaterials (Variables|/Script/Engine.StaticMeshActor|GetStaticMeshComponent _asstatic_mesh_actor) "Col" "0.400000,0.400000,0.400000")
      (else
        (Rendering|Material|SetVectorParameterValueonMaterials (Variables|/Script/Engine.StaticMeshActor|GetStaticMeshComponent _asstatic_mesh_actor) "Col" "0.000000,0.200000,1.000000")))
    (else
      (Rendering|Material|SetVectorParameterValueonMaterials (Variables|/Script/Engine.StaticMeshActor|GetStaticMeshComponent _asstatic_mesh_actor) "Col" "0.650000,0.000000,0.650000"))))

(fn OnRepHasPhysics)