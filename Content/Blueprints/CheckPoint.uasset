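; Checkpoint actor that updates the player's reset transform and lets them open a save menu.
; Overlapping its barrier stores the ThirdPersonCharacter's transform as ResetPos, shows a text render and enables input on the actor until overlap ends.
; Pressing E disables controller input, shows the cursor, writes an offset checkpoint position and the level name to GameInst, then opens the LoadSave widget.
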(event OnComponentBeginOverlap(CheckpointBarrier)
  (params (OverlappedComponent :type Primitive%20Component%20Object%20Reference) (OtherActor :type Actor%20Object%20Reference) (OtherComp :type Primitive%20Component%20Object%20Reference) (OtherBodyIndex :type Integer) (bFromSweep :type Boolean) (SweepResult :type Hit%20Result%20Structure%20%28by%20ref%29))
  (bind _asthird_person_character (Utilities|Casting|CastToThirdPersonCharacter OtherActor))
  (Variables|/Game/ThirdPersonBP/Blueprints/ThirdPersonCharacter.ThirdPersonCharacter_C|SetResetPos _asthird_person_character (Transformation|GetActorTransform _asthird_person_character))
  (Input|EnableInput (Game|GetPlayerController 0))
  (Rendering|SetVisibility (Variables|Default|GetTextRender) true false))

(event OnComponentEndOverlap(CheckpointBarrier)
  (params (OverlappedComponent :type Primitive%20Component%20Object%20Reference) (OtherActor :type Actor%20Object%20Reference) (OtherComp :type Primitive%20Component%20Object%20Reference) (OtherBodyIndex :type Integer))
  (Utilities|Casting|CastToThirdPersonCharacter OtherActor)
  (Input|DisableInput (Game|GetPlayerController 0))
  (Rendering|SetVisibility (Variables|Default|GetTextRender) false false))

(event EventBeginPlay)

(event Input|KeyboardEvents|E
  (params (Key :type Key%20Structure :default "None"))
  (bind _returnvalue (Game|GetPlayerController 0))
  (:Pressed
    (Input|DisableInput _returnvalue 0)
    (Variables|/Script/Engine.PlayerController|SetbShowMouseCursor _returnvalue true)
    (CallFunction|SaveMenu)))

(fn ConstructionScript)

(fn SaveMenu
  (bind _asgame_inst (Utilities|Casting|CastToGameInst (Game|GetGameInstance)))
  (Variables|/Game/Blueprints/GameInst.GameInst_C|SetPosition _asgame_inst (+ (Transformation|GetActorLocation) "0,100.000000, 0"))
  (bind _returnvalue (Game|GetCurrentLevelName true))
  (Variables|/Game/Blueprints/GameInst.GameInst_C|SetLevel _asgame_inst (Utilities|String|StringToName _returnvalue))
  (bind _returnvalue_2 (UserInterface|CreateWidget "/Game/UI/LoadSave.LoadSave_C"))
  (UserInterface|Viewport|AddtoViewport _returnvalue_2 0))