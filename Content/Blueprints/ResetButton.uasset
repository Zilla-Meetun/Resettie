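; Interactable reset button that, when E is pressed inside its trigger box, returns the player and puzzle objects to their start positions.
; Box overlap by the third-person character toggles input and an "E to interact" prompt.
; Pressing E resets the player, plus all tutorial cubes, wooden planks and icy blocks via their TransformableObjects.
; It also brightens a referenced spotlight and destroys a light barrier, if each is valid.
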(event OnComponentBeginOverlap(Box)
  (params (OverlappedComponent :type Primitive%20Component%20Object%20Reference) (OtherActor :type Actor%20Object%20Reference) (OtherComp :type Primitive%20Component%20Object%20Reference) (OtherBodyIndex :type Integer) (bFromSweep :type Boolean) (SweepResult :type Hit%20Result%20Structure%20%28by%20ref%29))
  (Utilities|Casting|CastToThirdPersonCharacter OtherActor)
  (Input|EnableInput (Game|GetPlayerController 0))
  (Rendering|SetVisibility (Variables|Default|GetEToInteract) true false))

(event OnComponentEndOverlap(Box)
  (params (OverlappedComponent :type Primitive%20Component%20Object%20Reference) (OtherActor :type Actor%20Object%20Reference) (OtherComp :type Primitive%20Component%20Object%20Reference) (OtherBodyIndex :type Integer))
  (Utilities|Casting|CastToThirdPersonCharacter OtherActor)
  (Input|DisableInput (Game|GetPlayerController 0))
  (Rendering|SetVisibility (Variables|Default|GetEToInteract) false false))

(event Input|KeyboardEvents|E
  (params (Key :type Key%20Structure :default "None"))
  (:Pressed
    (CallFunction|ResetPlayer)
    (CallFunction|ResetCubeTutorials)
    (CallFunction|ResetPlanks)
    (CallFunction|ResetIcy)
    (CallFunction|LightUp)
    (CallFunction|RemoveBarrier)))

(fn ConstructionScript)

(fn ResetCubeTutorials
  (bind _outactors (Actor|GetAllActorsOfClass "/Game/Blueprints/Cube_Tutorial.Cube_Tutorial_C"))
  (for _array_element _outactors
    (Default|ResetPos (Variables|/Game/Blueprints/Cube_Tutorial.Cube_Tutorial_C|GetTransformableObjects _array_element))))

(fn ResetPlayer
  (bind _asthird_person_character (Utilities|Casting|CastToThirdPersonCharacter (Game|GetPlayerCharacter 0)))
  (Default|ResetPosition _asthird_person_character))

(fn LightUp
  (bind _spotlight3 (Variables|Default|GetSpotLight3))
  (Utilities|IsValid _spotlight3
    (:Is%20Valid
      (Rendering|Components|Light|SetIntensity (Variables|/Script/Engine.Light|GetLightComponent _spotlight3) 5e+03))))

(fn RemoveBarrier
  (bind _lightbarrier (Variables|Default|GetLightBarrier))
  (Utilities|IsValid _lightbarrier
    (:Is%20Valid
      (Actor|DestroyActor _lightbarrier))))

(fn ResetPlanks
  (bind _outactors (Actor|GetAllActorsOfClass "/Game/Blueprints/WoodenPlank.WoodenPlank_C"))
  (for _array_element _outactors
    (Default|ResetPos (Variables|/Game/Blueprints/WoodenPlank.WoodenPlank_C|GetTransformableObjects _array_element))))

(fn ResetIcy
  (bind _outactors (Actor|GetAllActorsOfClass "/Game/Blueprints/IcyBlock.IcyBlock_C"))
  (for _array_element _outactors
    (Default|ResetPos (Variables|/Game/Blueprints/IcyBlock.IcyBlock_C|GetTransformableObjects _array_element))))