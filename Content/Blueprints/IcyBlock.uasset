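; IcyBlock is an ice block actor that the third-person character can interact with through an on-screen widget.
; When a character that is not holding anything enters its Box, it creates a CubeInterface widget, passes itself to it and hands the widget to the character.
; Leaving the Box removes the widget.
; When the mesh overlaps a DeathZone_Blueprint, it calls ResetPos on TransformableObjects to reset its position.
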(event OnComponentBeginOverlap(Box)
  (params (OverlappedComponent :type Primitive%20Component%20Object%20Reference) (OtherActor :type Actor%20Object%20Reference) (OtherComp :type Primitive%20Component%20Object%20Reference) (OtherBodyIndex :type Integer) (bFromSweep :type Boolean) (SweepResult :type Hit%20Result%20Structure%20%28by%20ref%29))
  (bind _asthird_person_character (Utilities|Casting|CastToThirdPersonCharacter OtherActor))
  (if (not (Variables|/Game/ThirdPersonBP/Blueprints/ThirdPersonCharacter.ThirdPersonCharacter_C|GetIsHolding _asthird_person_character))
    (bind _returnvalue (UserInterface|CreateWidget "/Game/UI/CubeInterface.CubeInterface_C"))
    (UserInterface|Viewport|AddtoViewport _returnvalue 0)
    (Default|GetActor _returnvalue self)
    (Default|GetInterfaceInst _asthird_person_character _returnvalue)))

(event OnComponentEndOverlap(Box)
  (params (OverlappedComponent :type Primitive%20Component%20Object%20Reference) (OtherActor :type Actor%20Object%20Reference) (OtherComp :type Primitive%20Component%20Object%20Reference) (OtherBodyIndex :type Integer))
  (Utilities|Casting|CastToThirdPersonCharacter OtherActor)
  (Utilities|IsValid (stale OnComponentBeginOverlap(Box) _returnvalue)
    (:Is%20Valid
      (Widget|RemovefromParent (stale OnComponentBeginOverlap(Box) _returnvalue)))))

(event OnComponentBeginOverlap(StaticMeshComponent)
  (params (OverlappedComponent :type Primitive%20Component%20Object%20Reference) (OtherActor :type Actor%20Object%20Reference) (OtherComp :type Primitive%20Component%20Object%20Reference) (OtherBodyIndex :type Integer) (bFromSweep :type Boolean) (SweepResult :type Hit%20Result%20Structure%20%28by%20ref%29))
  (Utilities|Casting|CastToDeathZone_Blueprint OtherActor)
  (Default|ResetPos (Variables|Default|GetTransformableObjects)))

(fn ConstructionScript)