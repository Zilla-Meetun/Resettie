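; Tutorial cube actor that offers a cube UI when the player comes near and respawns if it falls into a death zone.
; UIRange overlap removes the floating help text, creates a CubeInterface widget linked to the cube and character, and shows the mouse cursor, unless the character is holding something.
; Leaving the range closes the widget and hides the cursor.
; Mesh overlap with DeathZone_Blueprint resets position through TransformableObjects.
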(event OnComponentBeginOverlap(StaticMeshComponent)
  (params (OverlappedComponent :type Primitive%20Component%20Object%20Reference) (OtherActor :type Actor%20Object%20Reference) (OtherComp :type Primitive%20Component%20Object%20Reference) (OtherBodyIndex :type Integer) (bFromSweep :type Boolean) (SweepResult :type Hit%20Result%20Structure%20%28by%20ref%29))
  ;[1 1 1] Respawns Cube if dies
  (Utilities|Casting|CastToDeathZone_Blueprint OtherActor)
  (Default|ResetPos (Variables|Actor|GetTransformableObjects)))

(event OnComponentBeginOverlap(UIRange)
  (params (OverlappedComponent :type Primitive%20Component%20Object%20Reference) (OtherActor :type Actor%20Object%20Reference) (OtherComp :type Primitive%20Component%20Object%20Reference) (OtherBodyIndex :type Integer) (bFromSweep :type Boolean) (SweepResult :type Hit%20Result%20Structure%20%28by%20ref%29))
  ;[1 1 1] Overlap and end overlap events to open and close UI with refrence to physics object
  (bind _asthird_person_character (Utilities|Casting|CastToThirdPersonCharacter OtherActor))
  (if (not (Variables|/Game/ThirdPersonBP/Blueprints/ThirdPersonCharacter.ThirdPersonCharacter_C|GetIsHolding _asthird_person_character))
    (Utilities|IsValid (Variables|Default|GetHelpful%20Text)
      (:Is%20Valid
        (Components|DestroyComponent (Variables|Default|GetHelpful%20Text)))
      (:Is%20Not%20Valid
        _))
    (bind _returnvalue (UserInterface|CreateWidget "/Game/UI/CubeInterface.CubeInterface_C"))
    (UserInterface|Viewport|AddtoViewport _returnvalue 0)
    (Default|GetActor _returnvalue self)
    (Default|GetInterfaceInst _asthird_person_character _returnvalue)
    (Variables|/Script/Engine.PlayerController|SetbShowMouseCursor (Game|GetPlayerController 0) true)))

(event OnComponentEndOverlap(UIRange)
  (params (OverlappedComponent :type Primitive%20Component%20Object%20Reference) (OtherActor :type Actor%20Object%20Reference) (OtherComp :type Primitive%20Component%20Object%20Reference) (OtherBodyIndex :type Integer))
  ;[1 1 1] Overlap and end overlap events to open and close UI with refrence to physics object
  (Utilities|Casting|CastToThirdPersonCharacter OtherActor)
  (Utilities|IsValid (stale OnComponentBeginOverlap(UIRange) _returnvalue)
    (:Is%20Valid
      (Widget|RemovefromParent (stale OnComponentBeginOverlap(UIRange) _returnvalue))
      (Variables|/Script/Engine.PlayerController|SetbShowMouseCursor (Game|GetPlayerController 0) false))))

(event EventBeginPlay
  ;[1 1 1] Initalises Variable text
  (Rendering|Components|TextRender|SetText (Variables|Default|GetHelpful%20Text) (Variables|Default|GetHelpfulTxt)))

(fn ConstructionScript)